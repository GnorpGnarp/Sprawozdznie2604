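; BP_Jelly is a construction-time actor that pairs a scalable Jelly component with a column of instanced meshes.
; The construction script sets the Jelly's world scale from per-axis variables.
; It then stacks InstancedStaticMesh instances downward along local Z at fixed spacing, with the count derived from the length of the BottomEnd vector.
; The event graph holds only empty events, so the Blueprint adds no runtime logic.
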(event `self.Jelly.OnComponentHit`
  (params (HitComponent :type "PrimitiveComponent Object Reference") (OtherActor :type "Actor Object Reference") (OtherComp :type "PrimitiveComponent Object Reference") (NormalImpulse :type "Vector Structure") (Hit :type "HitResult Structure (by ref)")))

(fn `UserConstructionScript`
  (`SceneComponent.SetWorldScale3D` (`self.Jelly`) (`KismetMathLibrary.MakeVector` (`self.X_Scale`) (`self.Y_Scale`) (`self.Z_Scale`)))
  (`InstancedStaticMeshComponent.AddInstance` (`self.InstancedStaticMesh`) (`KismetMathLibrary.MakeTransform` (0.0 0.0 0.0)) false)
  (for _index (range (+ (`KismetMathLibrary.FTrunc` (/ (`KismetMathLibrary.VSize` (`self.BottomEnd`)) 55.0)) 1))
    (`InstancedStaticMeshComponent.AddInstance` (`self.InstancedStaticMesh`) (`KismetMathLibrary.MakeTransform` (`KismetMathLibrary.MakeVector` 0.0 0.0 (`KismetMathLibrary.Conv_IntToDouble` (* _index -130)))) false)))